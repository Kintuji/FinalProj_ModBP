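; AI controller that gathers all TargetPoint actors as waypoints on possess and runs behavior tree BP_BT1.
; Perception updates for BP_BaseCharacter actors write the seen actor and its location to the CanChase and HasKnownLoca Blackboard keys.
; Losing sight starts a short timer that clears only CanChase, and a new sighting cancels it.
; The hearing branch is an empty stub.
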(event `self.ReceivePossess`
  (params (PossessedPawn :type "Pawn Object Reference"))
  (bind _outactors (`GameplayStatics.GetAllActorsOfClass` "/Script/Engine.TargetPoint"))
  (set `self.waypoints` _outactors)
  (`self.RunBehaviorTree` "/Game/AI/BP_BT1.BP_BT1"))

(event `self.AIPerception.OnTargetPerceptionUpdated`
  (params (Actor :type "Actor Object Reference") (Stimulus :type "AIStimulus Structure"))
  (bind (_age _expirationage _strength _stimuluslocation _receiverlocation _tag _bsuccessfullysensed) (break `AIStimulus` Stimulus))
  (bind _blackboard (`self.Blackboard`))
  (cast `/Game/Blueprints/Player/BP_BaseCharacter` Actor)
  (bind _returnvalue (`AIPerceptionSystem.GetSenseClassForStimulus` Stimulus))
  (bind _asaisense_blueprint (castclass `AISense_Blueprint` _returnvalue))
  (if (== "/Script/AIModule.AISense_Sight" _asaisense_blueprint)
    (if _bsuccessfullysensed
      (`KismetSystemLibrary.K2_ClearAndInvalidateTimerHandle` (`self.loseSightHandle`))
      (`BlackboardComponent.SetValueAsObject` _blackboard (`self.CanChase`) Actor)
      (`BlackboardComponent.SetValueAsVector` _blackboard (`self.HasKnownLoca`) (`self.K2_GetActorLocation` Actor))
      (else
        (bind _returnvalue_2 (`KismetSystemLibrary.K2_SetTimerDelegate` (delegate `OnLoseSightConfirmed`) 1.0))
        (set `self.loseSightHandle` _returnvalue_2)))
    (elif (== _asaisense_blueprint "/Script/AIModule.AISense_Hearing")
      (if _bsuccessfullysensed
        _))))

(event `OnLoseSightConfirmed`
  (`BlackboardComponent.SetValueAsObject` (`self.Blackboard`) (`self.CanChase`) null))

(fn `UserConstructionScript`)