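; Base player controller that tracks collected wines and handles the player's death.
; On BeginPlay, the local controller adds the base Enhanced Input mapping context, binds to wine-collected and enemy-collided events, and sets game-only input with the cursor hidden.
; Each collected wine increments a counter.
; An enemy collision shows the game over widget and switches to UI-only input with a visible cursor.
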(event `self.ReceiveBeginPlay`
  (bind _returnvalue (subsystem `EnhancedInputLocalPlayerSubsystem`))
  (`parent.ReceiveBeginPlay`)
  (if (`self.IsLocalPlayerController`)
    (`|ExecutionSequence`
      (:`then_0`
        (`/Engine/EditorBlueprintResources/StandardMacros.IsValid` _returnvalue
          (:`Is Valid`
            (`EnhancedInputSubsystemInterface.AddMappingContext` _returnvalue "/Game/Input/IMC_BaseMapping.IMC_BaseMapping" 0 (struct)))))
      (:`then_1`
        (add `self.OnWineCollected` (delegate `AddWineCollected`)))
      (:`then_2`
        (add `self.OnEnemyCollided` (delegate `PlayerDied`))
        (`WidgetBlueprintLibrary.SetInputMode_GameOnly` self)
        (set `self.bShowMouseCursor` false)))))

(event `AddWineCollected`
  (set `self.Wines Collected` (+ 1 (`self.Wines Collected`))))

(event `PlayerDied`
  (`WidgetBlueprintLibrary.SetInputMode_GameOnly` self)
  (set `self.bShowMouseCursor` false)
  (bind _returnvalue (`|CreateWidget` "/Game/UI/W_GameOver.W_GameOver_C"))
  (`UserWidget.AddToViewport` _returnvalue 0)
  (`WidgetBlueprintLibrary.SetInputMode_UIOnlyEx` self _returnvalue)
  (set `self.bShowMouseCursor` true))

(fn `UserConstructionScript`)