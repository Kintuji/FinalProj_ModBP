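; BP_Wine is a collectible wine pickup that raises the player's drunkenness.
; Capsule overlap with a BP_BaseCharacter toggles an interact prompt widget and an in-range flag.
; The character's OnInteractE dispatcher, bound at BeginPlay, triggers collection when in range: it notifies BP_BaseController, plays a world camera shake, calls AddDrunkenness on the character's Wine component and destroys the actor.
; Tick prints current drunkenness as debug output.
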(event `self.Capsule.OnComponentBeginOverlap`
  (params (OverlappedComponent :type "PrimitiveComponent Object Reference") (OtherActor :type "Actor Object Reference") (OtherComp :type "PrimitiveComponent Object Reference") (OtherBodyIndex :type Integer) (bFromSweep :type Boolean) (SweepResult :type "HitResult Structure (by ref)"))
  (cast `/Game/Blueprints/Player/BP_BaseCharacter` OtherActor)
  (set `self.insideCollision` true)
  (bind _returnvalue (`|CreateWidget` "/Game/Widgets/W_Interact.W_Interact_C"))
  (bind _output_get (set `self.WidgetIntercat` _returnvalue))
  (`UserWidget.AddToViewport` _output_get 0))

(event `self.Capsule.OnComponentEndOverlap`
  (params (OverlappedComponent :type "PrimitiveComponent Object Reference") (OtherActor :type "Actor Object Reference") (OtherComp :type "PrimitiveComponent Object Reference") (OtherBodyIndex :type Integer))
  (cast `/Game/Blueprints/Player/BP_BaseCharacter` OtherActor)
  (set `self.insideCollision` false)
  (`Widget.RemoveFromParent` (`self.WidgetIntercat`)))

(event `self.ReceiveBeginPlay`
  (bind _asbp_base_character (cast `/Game/Blueprints/Player/BP_BaseCharacter` (`GameplayStatics.GetPlayerCharacter` 0)))
  (add `/Game/Blueprints/Player/BP_BaseCharacter.OnInteractE` _asbp_base_character (delegate `OnInteractE_Event`)))

(event `OnInteractE_Event`
  (if (`self.insideCollision`)
    (bind _asbp_base_controller (cast `/Game/Blueprints/Player/BP_BaseController` (`GameplayStatics.GetPlayerController` 0)))
    (`/Game/Blueprints/Player/BP_BaseController.OnWineCollected` _asbp_base_controller)
    (`GameplayStatics.PlayWorldCameraShake` "/Game/CameraVisual/CS_cameraShake.CS_cameraShake_C" (`self.K2_GetActorLocation`) 0.0 1500.0)
    (bind _asbp_base_character (cast `/Game/Blueprints/Player/BP_BaseCharacter` (`GameplayStatics.GetPlayerCharacter` 0)))
    (`WineComponent.AddDrunkenness` (`/Game/Blueprints/Player/BP_BaseCharacter.Wine` _asbp_base_character))
    (`self.K2_DestroyActor`)))

(event `self.ReceiveTick`
  (params (DeltaSeconds :type "Float (single-precision)"))
  (`KismetSystemLibrary.PrintString` (`KismetStringLibrary.Conv_DoubleToString` (`WineComponent.CurrentDrunkenness` (`/Game/Blueprints/Player/BP_BaseCharacter.Wine` (stale `OnInteractE_Event` _asbp_base_character))))))

(fn `UserConstructionScript`)