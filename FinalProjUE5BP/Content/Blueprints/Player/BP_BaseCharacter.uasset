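; BP_BaseCharacter is the player character Blueprint, handling Enhanced Input movement, look, sprint, jump and a pause menu.
; Movement follows control yaw, sprint switches max walk speed, and an IsJumping flag set on jump and cleared on landing blocks repeat jumps.
; The pause input creates the menu, pauses and shows the cursor.
; Its close branch reverses this but never clears the open flag, so the menu cannot reopen.
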(event `EnhancedInput|`
  (params (ActionValue :type Boolean) (ElapsedSeconds :type "Float (double-precision)") (TriggeredSeconds :type "Float (double-precision)"))
  (bind _returnvalue (`GameplayStatics.GetPlayerController` 0))
  (:`Started`
    (if (not (`self.IspauseMenuOpened?`))
      (set `self.IspauseMenuOpened?` true)
      (bind _returnvalue_2 (`|CreateWidget` null _returnvalue))
      (bind _output_get (set `self.PauseMenuWidget` _returnvalue_2))
      (`UserWidget.AddToViewport` _output_get 0)
      (`WidgetBlueprintLibrary.SetInputMode_GameAndUIEx` _returnvalue (`self.PauseMenuWidget`))
      (set `PlayerController.bShowMouseCursor` true (`GameplayStatics.GetPlayerController` 0))
      (`GameplayStatics.SetGamePaused` true)
      (else
        (set `self.IspauseMenuOpened?` (`self.IspauseMenuOpened`))
        (`Widget.RemoveFromParent` (`self.PauseMenuWidget`))
        (`GameplayStatics.SetGamePaused` false)
        (`WidgetBlueprintLibrary.SetInputMode_GameOnly` _returnvalue)
        (set `PlayerController.bShowMouseCursor` false (`GameplayStatics.GetPlayerController` 0))))))

(event `self.OnLanded`
  (params (Hit :type "HitResult Structure (by ref)"))
  (set `self.isJumping` false))

(event `self.OnJumped`
  (set `self.isJumping` true))

(event `EnhancedInput|/Game/Input/IA_Jump`
  (params (ActionValue :type Boolean) (ElapsedSeconds :type "Float (double-precision)") (TriggeredSeconds :type "Float (double-precision)") (InputAction :type "InputAction Object Reference" :default "/Game/Input/IA_Jump.IA_Jump"))
  (:`Triggered`
    (if (not (`self.isJumping`))
      (`self.Jump`)))
  (:`Completed`
    (`self.StopJumping`)))

(event `EnhancedInput|/Game/Input/IA_SprintOn`
  (params (ActionValue :type Boolean) (ElapsedSeconds :type "Float (double-precision)") (TriggeredSeconds :type "Float (double-precision)") (InputAction :type "InputAction Object Reference" :default "/Game/Input/IA_SprintOn.IA_SprintOn"))
  (:`Triggered`
    (bind _output_get (set `CharacterMovementComponent.MaxWalkSpeed` 1100.0 (`self.CharacterMovement`)))
    (`self.AddMovementInput` (0.0 0.0 0.0) _output_get)))

(event `EnhancedInput|/Game/Input/IA_SprintOff`
  (params (ActionValue :type Boolean) (ElapsedSeconds :type "Float (double-precision)") (TriggeredSeconds :type "Float (double-precision)") (InputAction :type "InputAction Object Reference" :default "/Game/Input/IA_SprintOff.IA_SprintOff"))
  (:`Triggered`
    (bind _output_get (set `CharacterMovementComponent.MaxWalkSpeed` 600.0 (`self.CharacterMovement`)))
    (`self.AddMovementInput` (0.0 0.0 0.0) _output_get)))

(event `EnhancedInput|/Game/Input/IA_Look`
  (params (ActionValue :type "Vector2D Structure") (ElapsedSeconds :type "Float (double-precision)") (TriggeredSeconds :type "Float (double-precision)") (InputAction :type "InputAction Object Reference" :default "/Game/Input/IA_Look.IA_Look"))
  (:`Triggered`
    (`self.AddControllerYawInput` ActionValue_X)
    (`self.AddControllerPitchInput` ActionValue_Y)))

(event `EnhancedInput|/Game/Input/IA_MoveForward`
  (params (ActionValue :type "Float (double-precision)") (ElapsedSeconds :type "Float (double-precision)") (TriggeredSeconds :type "Float (double-precision)") (InputAction :type "InputAction Object Reference" :default "/Game/Input/IA_MoveForward.IA_MoveForward"))
  (bind (_returnvalue_roll _returnvalue_pitch _returnvalue_yaw) (`KismetMathLibrary.BreakRotator` (`self.GetControlRotation`)))
  (:`Triggered`
    (`self.AddMovementInput` (`KismetMathLibrary.GetForwardVector` (`KismetMathLibrary.MakeRotator` 0.0 0.0 _returnvalue_yaw)) ActionValue)))

(event `EnhancedInput|/Game/Input/IA_MoveRight`
  (params (ActionValue :type "Float (double-precision)") (ElapsedSeconds :type "Float (double-precision)") (TriggeredSeconds :type "Float (double-precision)") (InputAction :type "InputAction Object Reference" :default "/Game/Input/IA_MoveRight.IA_MoveRight"))
  (bind (_returnvalue_roll _returnvalue_pitch _returnvalue_yaw) (`KismetMathLibrary.BreakRotator` (`self.GetControlRotation`)))
  (:`Triggered`
    (`self.AddMovementInput` (`KismetMathLibrary.GetRightVector` (`KismetMathLibrary.MakeRotator` 0.0 0.0 _returnvalue_yaw)) ActionValue)))

(fn `UserConstructionScript`)